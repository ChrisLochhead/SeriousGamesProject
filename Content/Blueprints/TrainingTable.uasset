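; Training table that lets the player open and close a training menu on the HUD while standing at it.
; Box overlap sets the main character's AtTable flag, which gates the ToggleTraining event.
; That event shows or hides the training menu and vector info panels, updating InTraining and the mouse cursor.
; Activation also snaps the control rotation to a fixed facing; an actor rotation node is left unconnected.
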(event `self.Box.OnComponentBeginOverlap`
  (params (OverlappedComponent :type "PrimitiveComponent Object Reference") (OtherActor :type "Actor Object Reference") (OtherComp :type "PrimitiveComponent Object Reference") (OtherBodyIndex :type Integer) (bFromSweep :type Boolean) (SweepResult :type "HitResult Structure (by ref)"))
  ;[1 1 1] Determine whether player is at the table or not
  (bind _asmain_character (cast `/Game/Blueprints/MainCharacter` OtherActor))
  (set `/Game/Blueprints/MainCharacter.atTable` true _asmain_character))

(event `self.Box.OnComponentEndOverlap`
  (params (OverlappedComponent :type "PrimitiveComponent Object Reference") (OtherActor :type "Actor Object Reference") (OtherComp :type "PrimitiveComponent Object Reference") (OtherBodyIndex :type Integer))
  ;[1 1 1] Determine whether player is at the table or not
  (bind _asmain_character (cast `/Game/Blueprints/MainCharacter` OtherActor))
  (set `/Game/Blueprints/MainCharacter.atTable` false _asmain_character))

(event `ToggleTraining`
  (params (Activate :type Boolean))
  (bind _returnvalue (`GameplayStatics.GetPlayerController` 0))
  ;[1 1 1] Toggle Training Menu on HUD
  (bind _asmain_character (cast `/Game/Blueprints/MainCharacter` (`GameplayStatics.GetPlayerCharacter` 0)))
  (if (`/Game/Blueprints/MainCharacter.atTable` _asmain_character)
    (bind _astraining_hud (cast `/Game/Blueprints/TrainingHUD` (`PlayerController.GetHUD` (`GameplayStatics.GetPlayerController` 0))))
    (if Activate
      (bind _hudwidget (`/Game/Blueprints/TrainingHUD.HUDWidget` _astraining_hud))
      (bind _trainingmenupanel (`/Game/Blueprints/TrainingMenuHUD.TrainingMenuPanel` _hudwidget))
      (`Widget.SetVisibility` _trainingmenupanel "Visible")
      (bind _vectorinfopanel (`/Game/Blueprints/TrainingMenuHUD.VectorInfoPanel` _hudwidget))
      (`Widget.SetVisibility` _vectorinfopanel "Visible")
      (bind _asmain_character_2 (cast `/Game/Blueprints/MainCharacter` (`GameplayStatics.GetPlayerCharacter` 0)))
      (set `/Game/Blueprints/MainCharacter.inTraining` true _asmain_character_2)
      (set `PlayerController.bShowMouseCursor` true _returnvalue)
      (`Controller.SetControlRotation` (`GameplayStatics.GetPlayerController` 0) (`KismetMathLibrary.MakeRotator` 0.0 0.0 90.0))
      (else
        (`Widget.SetVisibility` _trainingmenupanel "Hidden")
        (`Widget.SetVisibility` _vectorinfopanel "Hidden")
        (bind _asmain_character_3 (cast `/Game/Blueprints/MainCharacter` (`GameplayStatics.GetPlayerCharacter` 0)))
        (set `/Game/Blueprints/MainCharacter.inTraining` false _asmain_character_3)
        (set `PlayerController.bShowMouseCursor` false _returnvalue)))))

(fn `UserConstructionScript`)