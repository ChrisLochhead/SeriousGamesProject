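; A door Blueprint that swings open and closed on its yaw axis when triggered while the player is near.
; Box overlap events set a proximity flag and the MainCharacter's AtDoor flag, fetching player 0 without checking which actor overlapped.
; The openDoor event, gated on proximity, uses a FlipFlop to play or reverse a timeline that drives the door mesh's relative rotation.
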(event `self.Box.OnComponentBeginOverlap`
  (params (OverlappedComponent :type "PrimitiveComponent Object Reference") (OtherActor :type "Actor Object Reference") (OtherComp :type "PrimitiveComponent Object Reference") (OtherBodyIndex :type Integer) (bFromSweep :type Boolean) (SweepResult :type "HitResult Structure (by ref)"))
  ;[1 1 1] Check if near door
  (set `self.isNear` true)
  (bind _asmain_character (cast `/Game/MainCharacter` (`GameplayStatics.GetPlayerCharacter` 0)))
  (set `/Game/MainCharacter.atDoor` true _asmain_character))

(event `self.Box.OnComponentEndOverlap`
  (params (OverlappedComponent :type "PrimitiveComponent Object Reference") (OtherActor :type "Actor Object Reference") (OtherComp :type "PrimitiveComponent Object Reference") (OtherBodyIndex :type Integer))
  ;[1 1 1] Check if near door
  (set `self.isNear` false)
  (bind _asmain_character (cast `/Game/MainCharacter` (`GameplayStatics.GetPlayerCharacter` 0)))
  (set `/Game/MainCharacter.atDoor` false _asmain_character))

(event `openDoor`
  ;[1 1 1] Door Rotation
  (if (`self.isNear`)
    (`/Engine/EditorBlueprintResources/StandardMacros.FlipFlop`
      (:`A`
        (bind (_direction _doorrot) (`Timeline|DoorRotation` :!label _label)
          (:`Update`
            (`SceneComponent.K2_SetRelativeRotation` (`self.SM_Door`) (`KismetMathLibrary.MakeRotator` 0.0 0.0 _doorrot) false false))))
      (:`B`
        (goto _label :!via `Reverse`)))))

(fn `UserConstructionScript`)