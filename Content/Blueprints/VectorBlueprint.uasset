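; VectorBlueprint is an actor with a static mesh that takes player input and tracks whether the left mouse button is held.
; BeginPlay enables input from player controller 0, and left mouse press and release set LMBPressed.
; Logic to roll the actor by mouse X while pressed exists but is disconnected, so it never runs.
; A DestroySelf function destroys the actor, while Tick and the construction script are empty.
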(event `self.ReceiveBeginPlay`
  ;[1 1 1] Activate input for this player
  (`self.EnableInput` (`GameplayStatics.GetPlayerController` 0)))

(event `self.ReceiveTick`
  (params (DeltaSeconds :type "Float (single-precision)")))

(event `Key|LeftMouseButton`
  (params (Key :type "Key Structure"))
  ;[1 1 1] Set LMBPressed variable
  (:`Pressed`
    (set `self.LMBPressed` true))
  (:`Released`
    (set `self.LMBPressed` false)))

(fn `DestroySelf`
  (`self.K2_DestroyActor`))

(fn `UserConstructionScript`)