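; TrainingHUD switches the player's screen between the training menu and note widgets.
; BeginPlay creates both widgets once, stores them and shows the training menu.
; Tick polls MainCharacter: an active note or test swaps in the note widget, and the menu returns when neither is active.
; An IsNote flag limits each swap to state changes, clearing all widgets before adding the new one.
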(event `self.ReceiveBeginPlay`
  (bind _returnvalue (`|CreateWidget` "/Game/Blueprints/NoteHUD.NoteHUD_C"))
  (bind _output_get (set `self.NoteWidget` _returnvalue))
  (bind _returnvalue_2 (`|CreateWidget` "/Game/Blueprints/TrainingMenuHUD.TrainingMenuHUD_C"))
  (set `self.HUDWidget` _returnvalue_2)
  (`UserWidget.AddToViewport` _returnvalue_2 0 :!label _label))

(event `self.ReceiveTick`
  (params (DeltaSeconds :type "Float (single-precision)"))
  (bind _isnote (`self.isNote`))
  (bind _asmain_character (cast `/Game/Blueprints/MainCharacter` (`GameplayStatics.GetPlayerCharacter` 0)))
  (if (`/Game/Blueprints/MainCharacter.NoteActive` _asmain_character)
    (if (not _isnote) :!label _label_2
      (set `self.isNote` true)
      (`WidgetLayoutLibrary.RemoveAllWidgets`)
      (`UserWidget.AddToViewport` (stale `self.ReceiveBeginPlay` _output_get) 0))
    (elif (`/Game/Blueprints/MainCharacter.inTest` _asmain_character)
      (goto _label_2)
      (elif _isnote
        (set `self.isNote` false)
        (`WidgetLayoutLibrary.RemoveAllWidgets`)
        (goto _label)))))

(fn `UserConstructionScript`)