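; Player character Blueprint with first-person style movement and look, frozen during training, plus interaction with notes and a training table.
; Each tick a camera line trace checks for a target actor class, destroying it while G is held, and control pitch sets whether the player looks at the table.
; Overlapping a Note stores its index, and E flags the note view active when looking at the table.
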(event `InputAxis|Forward/Backward`
  (params (AxisValue :type "Float (single-precision)"))
  ;[1 1 1] Movement and camera controls
  (if (not (`self.inTraining`))
    (`self.AddMovementInput` (`KismetMathLibrary.GetForwardVector` (`KismetMathLibrary.MakeRotator` 0.0 0.0 (.yaw (`self.GetControlRotation`)))) AxisValue)))

(event `InputAxis|Left/Right`
  (params (AxisValue :type "Float (single-precision)"))
  ;[1 1 1] Movement and camera controls
  (if (not (`self.inTraining`))
    (`self.AddMovementInput` (`KismetMathLibrary.GetRightVector` (`KismetMathLibrary.MakeRotator` 0.0 0.0 (.yaw (`self.GetControlRotation`)))) AxisValue)))

(event `InputAxis|MouseX`
  (params (AxisValue :type "Float (single-precision)"))
  ;[1 1 1] Movement and camera controls
  (if (not (`self.inTraining`))
    (`self.AddControllerYawInput` AxisValue)))

(event `InputAxis|MouseY`
  (params (AxisValue :type "Float (single-precision)"))
  ;[1 1 1] Movement and camera controls
  (if (not (`self.inTraining`))
    (`self.AddControllerPitchInput` (* AxisValue -1.0))))

(event `self.ReceiveTick`
  (params (DeltaSeconds :type "Float (single-precision)"))
  (bind _pitch (.pitch (`self.GetControlRotation` (`GameplayStatics.GetPlayerCharacter` 0))))
  (bind (_is_hit _hit_object) (`self.doesIntersect` (`self.Empty2`)))
  (set `self.hitObject` _hit_object)
  (if _is_hit
    (if (and (`self.interactPressed`) (!= (`self.hitObject`) null))
      (`self.K2_DestroyActor` (`self.hitObject`))
      ;[1 1 1] Determine whether player has the right forward vector for the training menu
      (if (> 15.0 _pitch) :!label _label
        (set `self.isLookingAtTable` true :!label _label_2)
        (elif (> _pitch 330.0)
          (goto _label_2)
          (else
            (set `self.isLookingAtTable` false)))))
    (else
      (goto _label))))

(event `self.ReceiveBeginPlay`
  ;[1 1 1] Initialise variables
  (set `self.AccessLevel` 1)
  (set `self.atDoor` false)
  (set `self.atTable` false)
  (set `self.inTraining` false)
  (set `self.isLookingAtTable` false))

(event `Key|G`
  (params (Key :type "Key Structure"))
  (:`Pressed`
    (set `self.interactPressed` true))
  (:`Released`
    (set `self.interactPressed` false)))

(event `self.ReceiveActorBeginOverlap`
  (params (OtherActor :type "Actor Object Reference"))
  (bind _asnote (cast `/Game/Blueprints/Note` OtherActor)
    (:`then`
      (set `self.Current Note` (`/Game/Blueprints/Note.NoteIndex` _asnote))
      (set `self.isLookingAtNote` true))
    (:`CastFailed`
      (set `self.isLookingAtNote` false))))

(event `Key|E`
  (params (Key :type "Key Structure"))
  (:`Pressed`
    (if (`self.isLookingAtTable`)
      (set `self.NoteActive` true))))

(fn `doesIntersect`
  (params (`Object Type` :type "Actor Class Reference"))
  (returns (`Is Hit` :type Boolean) (`Hit Object` :type "Actor Object Reference"))
  (locals (CompareObject :type "Actor Object Reference") (Hit :type Boolean) (Type :type "Actor Class Reference"))
  (bind _returnvalue (`GameplayStatics.GetPlayerCameraManager` 0))
  (bind _returnvalue_2 (`self.K2_GetActorLocation` _returnvalue))
  (bind _output_get (set `local.Type` `Object Type`))
  (if (!= _output_get null)
    (bind _outhit (`KismetSystemLibrary.LineTraceSingle` _returnvalue_2 (+ _returnvalue_2 (* (`self.GetActorForwardVector` _returnvalue) 500)) "TraceTypeQuery1"))
    (bind _output_get_2 (set `local.CompareObject` (`.HitActor` (`GameplayStatics.BreakHitResult` _outhit))))
    (if (== (`local.Type`) (`GameplayStatics.GetObjectClass` _output_get_2))
      (return true (`local.CompareObject`))
      (else
        (return false (`local.CompareObject`))))
    (else
      (`KismetSystemLibrary.PrintString` "Class is null"))))

(fn `ToggleViewNote`)

(fn `UserConstructionScript`)